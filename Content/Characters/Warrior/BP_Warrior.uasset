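; BP_Warrior is a warrior character that can show a widget for a timed yell.
; Each Tick turns its Scene component on yaw only to face the camera of the BP_PlayerWarlord player pawn.
; Yell shows the widget, prints a placeholder "Hello" and hides the widget after Duration; its Message input is unused.
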(event `self.ReceiveTick`
  (params (DeltaSeconds :type "Float (single-precision)"))
  (bind _asbp_player_warlord (cast `/Game/Player/BP_PlayerWarlord` (`GameplayStatics.GetPlayerPawn` 0)))
  (bind (_returnvalue_roll _returnvalue_pitch _returnvalue_yaw) (`KismetMathLibrary.BreakRotator` (`KismetMathLibrary.FindLookAtRotation` (`SceneComponent.K2_GetComponentLocation` (`self.Scene`)) (`SceneComponent.K2_GetComponentLocation` (`/Game/Player/BP_PlayerWarlord.Camera` _asbp_player_warlord)))))
  (`SceneComponent.K2_SetWorldRotation` (`self.Scene`) (`KismetMathLibrary.MakeRotator` 0.0 0.0 _returnvalue_yaw) false false))

(event `Yell`
  (params (Message :type String) (Duration :type "Float (double-precision)"))
  (bind _widget (`self.Widget`))
  (`SceneComponent.SetVisibility` _widget true false)
  (`KismetSystemLibrary.PrintString` "Hello")
  (`KismetSystemLibrary.Delay` Duration)
  (`SceneComponent.SetVisibility` _widget false false))

(fn `UserConstructionScript`)
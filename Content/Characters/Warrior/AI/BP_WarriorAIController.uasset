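; AI controller for BP_Warrior pawns that runs their behavior tree and picks their combat target.
; On possess it caches the warrior, starts BT_Warrior and writes the warrior's Allegiance to the Blackboard, printing an error for other pawn types.
; AI Perception updates feed UpdateTarget, which, while the warrior has no valid target, stores perceived BP_Warlord actors as Target on the pawn, without an allegiance check.
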(event `self.ReceivePossess`
  (params (PossessedPawn :type "Pawn Object Reference"))
  (bind _asbp_warrior (cast `/Game/Characters/Warrior/BP_Warrior` PossessedPawn)
    (:`then`
      (set `self.StoredWarrior` _asbp_warrior)
      (`self.RunBehaviorTree` "/Game/Characters/Warrior/AI/BT_Warrior.BT_Warrior")
      (`BlackboardComponent.SetValueAsEnum` (`AIBlueprintHelperLibrary.GetBlackboard` self) "Allegiance" (`/Game/Characters/Warrior/BP_Warrior.Allegiance` (`self.StoredWarrior`))))
    (:`CastFailed`
      (`KismetSystemLibrary.PrintString` "Error: Owning pawn must be of BP_Warrior type" true true (struct :`R` 1.0 :`A` 1.0) 10.0))))

(event `self.AIPerception.OnPerceptionUpdated`
  (params (UpdatedActors :type "Array of Actor Object Reference (by ref)"))
  (`self.UpdateTarget` UpdatedActors))

(fn `UpdateTarget`
  (params (Array :type "Array of Actor Object Reference"))
  (locals (CurrentTarget :type "Actor Object Reference"))
  (if (not (`KismetSystemLibrary.IsValid` (`/Game/Characters/Warrior/BP_Warrior.Target` (`self.StoredWarrior`))))
    (for _array_element Array
      (bind _asbp_warlord (cast `/Game/Characters/Warlord/BP_Warlord` _array_element))
      (set `/Game/Characters/Warrior/BP_Warrior.Target` _asbp_warlord (`self.StoredWarrior`)))))

(fn `UserConstructionScript`)
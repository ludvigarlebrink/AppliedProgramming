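; BP_Water is a water surface actor that tiles a water mesh into a configurable ComponentsX by ComponentsY grid.
; The construction script adds an SM_Water63x63 static mesh component per cell at 63-unit spacing, with shadow casting off and enlarged bounds.
; The event graph has no active logic.
; A CreateComponent helper adds a procedural mesh component at an offset, but the construction script does not call it.
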(fn `CreateComponent`
  (params (Offset :type "Vector Structure"))
  (`AddComponent|NODE_AddProceduralMeshComponent-0` :`RelativeTransform` (`KismetMathLibrary.Conv_VectorToTransform` Offset)))

(fn `UserConstructionScript`
  (for _index (range (`self.ComponentsX`))
    (for _index_2 (range (`self.ComponentsY`))
      (bind _returnvalue (`AddComponent|NODE_AddStaticMeshComponent-1` :`RelativeTransform` (`KismetMathLibrary.Conv_VectorToTransform` (`KismetMathLibrary.MakeVector` (`KismetMathLibrary.Conv_IntToDouble` (* _index 63)) (`KismetMathLibrary.Conv_IntToDouble` (* _index_2 63))))))
      (`StaticMeshComponent.SetStaticMesh` _returnvalue "/Game/Meshes/Water/SM_Water63x63.SM_Water63x63")
      (`PrimitiveComponent.SetCastShadow` _returnvalue false)
      (`PrimitiveComponent.SetBoundsScale` _returnvalue 2.0))))
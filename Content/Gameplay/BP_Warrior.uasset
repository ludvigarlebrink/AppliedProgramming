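; BP_Warrior is a warrior actor that follows a Target and can swing a sword and jump.
; Each tick it teleports a step toward the Target at MovementSpeed without sweeping, keeping the Sphere's height, until it is within a small distance.
; OnAttack plays the SwordAttack timeline to pitch the Scene1 component, while OnJump applies a large upward force to the Sphere.
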(event `self.ReceiveTick`
  (params (DeltaSeconds :type "Float (single-precision)"))
  (bind _returnvalue (`SceneComponent.K2_GetComponentLocation` (`self.Target`)))
  (bind _returnvalue_2 (`SceneComponent.K2_GetComponentLocation` (`self.Sphere`)))
  (if (`KismetSystemLibrary.IsValid` (`self.Target`))
    (if (> (`KismetMathLibrary.Vector_Distance` _returnvalue _returnvalue_2) 10.0)
      (`self.K2_SetActorLocation` (`KismetMathLibrary.MakeVector` (.x (+ (* (`KismetMathLibrary.Normal` (- _returnvalue _returnvalue_2)) (* DeltaSeconds (`self.MovementSpeed`))) _returnvalue_2)) (.y (+ (* (`KismetMathLibrary.Normal` (- _returnvalue _returnvalue_2)) (* DeltaSeconds (`self.MovementSpeed`))) _returnvalue_2)) (.z _returnvalue_2)) false true))))

(event `OnAttack`
  (bind (_direction _swordattack) (`Timeline|SwordAttack` :!via `PlayFromStart`)
    (:`Update`
      (`SceneComponent.K2_SetRelativeRotation` (`self.Scene1`) (`KismetMathLibrary.MakeRotator` 0.0 (* _swordattack 90.0)) false false))))

(event `OnJump`
  (`PrimitiveComponent.AddForce` (`self.Sphere`) (0.0 0.0 7000000.0) "None" false))

(fn `UserConstructionScript`)